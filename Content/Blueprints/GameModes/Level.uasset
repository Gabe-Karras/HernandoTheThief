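; Level game mode Blueprint that manages the player's on-screen UI and death screen.
; On BeginPlay it creates the PlayerUI widget, adds it to the viewport and stores a reference.
; Custom events show or hide that widget's canvas, and CreateDeathScreen hides it before adding a new DeathScreen widget to the viewport.
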(event `self.ReceiveBeginPlay`
  (`self.CreateUI`))

(event `CreateUI`
  ; Spawn player UI widget
  (bind _returnvalue (`|CreateWidget` "/Game/Blueprints/Widgets/Screens/PlayerUI.PlayerUI_C"))
  (`UserWidget.AddToViewport` _returnvalue 0)
  (set `self.PlayerUI` _returnvalue))

(event `CreateDeathScreen`
  ; Remove UI and spawn death screen
  (`self.DisableUI`)
  (bind _returnvalue (`|CreateWidget` "/Game/Blueprints/Widgets/Screens/DeathScreen.DeathScreen_C"))
  (`UserWidget.AddToViewport` _returnvalue 0))

(event `DisableUI`
  ; Make UI invisible
  (set `Widget.Visibility` "Hidden" (`/Game/Blueprints/Widgets/Screens/PlayerUI.Canvas` (`self.PlayerUI`))))

(event `EnableUI`
  ; Make UI visible
  (set `Widget.Visibility` "Visible" (`/Game/Blueprints/Widgets/Screens/PlayerUI.Canvas` (`self.PlayerUI`))))

(fn `UserConstructionScript`)