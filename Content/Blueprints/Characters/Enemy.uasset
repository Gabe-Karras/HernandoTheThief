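; Enemy character that chases the player on sight and deals melee damage.
; PawnSensing triggers FollowPlayer, which uses AIMoveTo toward player 0 while they are alive and calls Attack on arrival.
; Attack plays a montage, then applies Damage through the player's UpdateHp after a short delay without rechecking range.
; CanAttack toggles around that delay but is never checked in this graph.
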(event `self.ReceiveBeginPlay`
  (set `CharacterMovementComponent.MaxWalkSpeed` (`self.Speed`) (`self.CharacterMovement`)))

(event `self.PawnSensing.OnSeePawn`
  (params (Pawn :type "Pawn Object Reference"))
  (`self.FollowPlayer`))

(event `FollowPlayer`
  (bind _returnvalue (`GameplayStatics.GetPlayerCharacter` 0))
  ; Chase player while the enemy is in a nav mesh, attack when reaching player if player is alive
  (bind _asplayer (cast `/Game/Blueprints/Characters/Player` _returnvalue))
  (if (not (`/Game/Blueprints/Characters/Player.IsDead` _asplayer))
    (`|AIMoveTo` self (0.0 0.0 0.0) _returnvalue 70.0
      (:`OnSuccess`
        (`self.Attack`)))))

(event `Attack`
  ; Play attack animation and inflict damage
  (`|PlayMontage` (`self.Mesh`) (`self.AttackAnim`)
    (:`then`
      (set `self.CanAttack` false)
      (`KismetSystemLibrary.Delay` 0.2)
      (set `self.CanAttack` true)
      (bind _asplayer (cast `/Game/Blueprints/Characters/Player` (`GameplayStatics.GetPlayerCharacter` 0)))
      (`/Game/Blueprints/Characters/Player.UpdateHp` _asplayer (`self.Damage`)))))

(fn `UserConstructionScript`)