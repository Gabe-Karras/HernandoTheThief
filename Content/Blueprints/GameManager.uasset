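; Game manager that tracks collected crystals and unlocks the player's spells as the count reaches set benchmarks.
; CollectCrystal records each crystal ID, updates the count and unlocks Fireball, Jump and Obliterate in sequence on exact benchmark matches.
; GetCurrentBenchmark returns the first benchmark above the count with its matching spell icon, or zero once all benchmarks are reached.
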(event `CollectCrystal`
  (params (Id :type Integer))
  (bind _collectedcrystals (`self.CollectedCrystals`))
  ; Add crystal ID and update count. Unlock spells when benchmarks are hit
  (`KismetArrayLibrary.Array_Add` _collectedcrystals Id)
  (bind _output_get (set `self.NumCrystals` (`KismetArrayLibrary.Array_Length` _collectedcrystals)))
  (if (`self.FireballUnlocked`)
    (if (`self.JumpUnlocked`)
      (if (`self.ObliterateUnlocked`)
        _
        (elif (== _output_get (`|GetArrayItem` (`self.SpellBenchmarks`) 2))
          (set `self.ObliterateUnlocked` true)))
      (elif (== _output_get (`|GetArrayItem` (`self.SpellBenchmarks`) 1))
        (set `self.JumpUnlocked` true)))
    (elif (== _output_get (`|GetArrayItem` (`self.SpellBenchmarks`)))
      (set `self.FireballUnlocked` true))))

(fn `GetCurrentBenchmark`
  (returns (CurrentBenchmark :type Integer) (Icon :type "Texture2D Object Reference"))
  ; Get the current crystal benchmark and icon for the next spell. Return 0 if all spells are unlocked
  (for (_array_element _array_index) (`self.SpellBenchmarks`)
    (if (< (`self.NumCrystals`) _array_element)
      (bind _output (`|GetArrayItem` (`self.SpellIcons`) _array_index))
      (return _array_element _output)))
  (return 0 _output))