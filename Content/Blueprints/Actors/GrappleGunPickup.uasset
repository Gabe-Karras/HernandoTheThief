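; Pickup actor that grants the player the grapple gun.
; On overlap with the Player, it sets the GrappleGunUnlocked flag on the GameManager game instance and destroys itself.
; On BeginPlay it checks that same flag and removes itself if the gun is already unlocked, so the pickup does not reappear once collected.
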(event `self.ReceiveBeginPlay`
  (bind _asgame_manager (cast `/Game/Blueprints/GameManager` (`GameplayStatics.GetGameInstance`)))
  (if (`/Game/Blueprints/GameManager.GrappleGunUnlocked` _asgame_manager)
    (`self.K2_DestroyActor`)))

(event `self.ReceiveActorBeginOverlap`
  (params (OtherActor :type "Actor Object Reference"))
  (cast `/Game/Blueprints/Characters/Player/Player` OtherActor)
  (bind _asgame_manager (cast `/Game/Blueprints/GameManager` (`GameplayStatics.GetGameInstance`)))
  (set `/Game/Blueprints/GameManager.GrappleGunUnlocked` true _asgame_manager)
  (`self.K2_DestroyActor`))

(fn `UserConstructionScript`)