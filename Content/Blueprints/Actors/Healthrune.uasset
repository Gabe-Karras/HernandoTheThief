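; Healthrune is a one-time collectible actor whose collected state is tracked by Id in the GameManager game instance.
; On BeginPlay it destroys itself if its Id is already in CollectedCrystals.
; When a Player overlaps it, it adds its Id to that collection and destroys itself, with no health effect applied here.
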(event `self.ReceiveBeginPlay`
  ; Destroy on spawn if this crystal has already been collected
  (bind _asgame_manager (cast `/Game/Blueprints/GameManager` (`GameplayStatics.GetGameInstance`)))
  (if (`KismetArrayLibrary.Array_Contains` (`/Game/Blueprints/GameManager.CollectedCrystals` _asgame_manager) (`self.Id`))
    (`self.K2_DestroyActor`)))

(event `self.ReceiveActorBeginOverlap`
  (params (OtherActor :type "Actor Object Reference"))
  ; When touched by player, mark as collected and destroy
  (cast `/Game/Blueprints/Characters/Player/Player` OtherActor)
  (bind _asgame_manager (cast `/Game/Blueprints/GameManager` (`GameplayStatics.GetGameInstance`)))
  (`KismetArrayLibrary.Array_Add` (`/Game/Blueprints/GameManager.CollectedCrystals` _asgame_manager) (`self.Id`))
  (`self.K2_DestroyActor`))

(fn `UserConstructionScript`)